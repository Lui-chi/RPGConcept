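; BP_Item is an item actor that shows an equip prompt when an RPGConceptCharacter overlaps it.
; Begin overlap sets the character's isOverlappingItem flag, creates a WBP_EquipItemPromt, passes it to SetCorrectItemName and adds it to the viewport.
; End overlap clears the flag and removes every top-level prompt widget of that class.
; SetCorrectItemName is empty here, apparently a hook for child items to name the prompt.
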(event EventBeginPlay)

(event Collision|EventActorBeginOverlap
  (params (OtherActor :type Actor%20Object%20Reference))
  (bind _asrpgconcept_character (Utilities|Casting|CastToRPGConceptCharacter OtherActor))
  (Class|RPGConceptCharacter|SetisOverlappingItem _asrpgconcept_character true)
  (bind _returnvalue (UserInterface|CreateWidget "/Game/Blueprint/HUD/WBP_EquipItemPromt.WBP_EquipItemPromt_C"))
  (CallFunction|SetCorrectItemName _returnvalue)
  (UserInterface|Viewport|AddtoViewport _returnvalue 0))

(event EventTick
  (params (DeltaSeconds :type Float%20%28single-precision%29)))

(event Collision|EventActorEndOverlap
  (params (OtherActor :type Actor%20Object%20Reference))
  (bind _asrpgconcept_character (Utilities|Casting|CastToRPGConceptCharacter OtherActor))
  (Class|RPGConceptCharacter|SetisOverlappingItem _asrpgconcept_character false)
  (bind _foundwidgets (Widget|GetAllWidgetsOfClass "/Game/Blueprint/HUD/WBP_EquipItemPromt.WBP_EquipItemPromt_C" true))
  (for _array_element _foundwidgets
    (Widget|RemovefromParent _array_element)))

(fn ConstructionScript)

(fn SetCorrectItemName
  (params (Widget%20Reference :type WBP%20Equip%20Item%20Promt%20Object%20Reference)))